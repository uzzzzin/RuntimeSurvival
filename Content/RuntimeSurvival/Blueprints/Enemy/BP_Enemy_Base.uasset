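; BP_Enemy_Base is the base enemy, which deals contact damage when it overlaps the player pawn.
; InitEnemy copies its EnemyID row from the game instance's data table into RuntimeStats, setting health and walk speed.
; Pool handlers toggle visibility, collision and tick, re-running InitEnemy on activation at the given location.
; GoDie spawns an experience orb carrying the reward, notifies the killer and unregisters from the interface-found spawn manager.
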(event EventBeginPlay
  (bind _outactors (Actor|GetAllActorswithInterface "/Game/RuntimeSurvival/Core/Interface/BPI_CanManageEnemySpawn.BPI_CanManageEnemySpawn_C"))
  (Variables|Default|SetEnemySpawnManager (Utilities|Array|Get(acopy) _outactors))
  (CallFunction|InitEnemy))

(event Collision|EventActorBeginOverlap
  (params (OtherActor :type Actor%20Object%20Reference))
  ;[0.15 0.15 0.15 0.5] Enemy와 Player가 충돌한다면.. Player는 무조건 데미지를 입음
  (if (== OtherActor (Game|Player|GetPlayerPawn 0))
    (Class|BPIDamageable|TakeDamage(Message) OtherActor self (Math|Float|Truncate (.finalcontactdamage (Variables|Default|GetRuntimeStats))))))

(event EventTick
  (params (DeltaSeconds :type Float%20%28single-precision%29)))

(event EventHandlePoolDeactivated
  (Rendering|SetActorHiddenInGame true)
  (Collision|SetActorEnableCollision false)
  (Actor|Tick|SetActorTickEnabled false))

(event EventHandlePoolActivated
  (params (InLocation :type Vector :default "0, 0, 0"))
  (bind _bpc_poolablecomponent (Variables|Default|GetBPC_PoolableComponent))
  (Variables|/Game/RuntimeSurvival/Blueprints/PoolSystem/BPC_PoolableComponent.BPC_PoolableComponent_C|SetInitLoc _bpc_poolablecomponent InLocation)
  (Transformation|SetActorLocation (Variables|/Game/RuntimeSurvival/Blueprints/PoolSystem/BPC_PoolableComponent.BPC_PoolableComponent_C|GetInitLoc _bpc_poolablecomponent) false false)
  (Rendering|SetActorHiddenInGame false)
  (Collision|SetActorEnableCollision true)
  (Actor|Tick|SetActorTickEnabled true)
  (CallFunction|InitEnemy))

(event EventGoDie
  (params (InKiller :type Actor%20Object%20Reference))
  (bind _returnvalue (Transformation|GetActorLocation))
  ;[0.15 0.15 0.15 0.5] Enemy가 죽을 때, Enemy의 위치에 ExpOrb를 스폰하고 Enemy가 들고 있는 경험치숫자를 스폰하는 ExpOrb에 넘겨줌.
  (bind _returnvalue_2 (Game|SpawnActorfromClass "/Game/RuntimeSurvival/Blueprints/Dropped/BP_ExpOrb.BP_ExpOrb_C" (Math|Conversions|ToTransform(Vector) (Math|Vector|MakeVector (.x _returnvalue) (.y _returnvalue) (Variables|Default|GetExpSpawnLocationZ))) "AlwaysSpawn" "MultiplyWithRoot" 0 0))
  (Default|SetExp _returnvalue_2 (.finalexpreward (Variables|Default|GetRuntimeStats)))
  ;[0.15 0.15 0.15 0.5] Player가 Enemy를 처치했다는 걸 플레이어에게 알려줌
  (Class|BPIPlayerKillEnemyEvent|NotifyPlayerKillEnemy(Message) InKiller (Transformation|GetActorLocation))
  (Class|BPICanManageEnemySpawn|UnregisterSpawnedEnemyInterface(Message) (Variables|Default|GetEnemySpawnManager) self))

(fn ConstructionScript)

(fn InitEnemy
  ;[0.15 0.15 0.15 0.5] 나중에 뺄 코드...
  (bind _outenemydata (Class|BPICanProvideGameData|GetEnemyData(Message) (Game|GetGameInstance)))
  (bind _returnvalue (Utilities|GetDataTableRow _outenemydata (Variables|Default|GetEnemyID))
    (:then
      (bind _output_get (LocalVariables|SetTempEnemyStat _returnvalue))
      (Variables|Default|SetRuntimeStats (Utilities|Struct|MakeST_RuntimeEnemyStat (.basemaxhealth _output_get) (.basemovespeed _output_get) (.basecontactdamage _output_get) (.baseattackdamage _output_get) (.baseattackcooldown _output_get) (.baseattackrange _output_get) (.expreward _output_get)))
      ;[0.15 0.15 0.15 0.5] EnemyBase 변수 세팅
      (Variables|Default|SetCurHealth (.finalmaxhealth (Variables|Default|GetRuntimeStats)))
      (Variables|/Script/Engine.CharacterMovementComponent|SetMaxWalkSpeed (Variables|Character|GetCharacterMovement) (.finalmovespeed (Variables|Default|GetRuntimeStats)))
      (Variables|Default|SetbIsDead false))))

(fn IsDead
  (return (Variables|Default|GetbIsDead)))

(fn IsEnemy
  (return true))