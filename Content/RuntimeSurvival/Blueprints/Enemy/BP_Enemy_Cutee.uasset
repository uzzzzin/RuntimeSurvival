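; BP_Enemy_Cutee is a pooled enemy for the survival game, built on a parent enemy class.
; It deals its final contact damage when its capsule overlaps a component tagged PlayerDamageBody, and loses health only to hits from player pawn 0.
; On death it sets a dead flag for the animation, waits briefly, runs the parent death logic, returns to the pool and clears the flag for respawn.
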(event OnComponentBeginOverlap(CapsuleComponent)
  (params (OverlappedComponent :type Primitive%20Component%20Object%20Reference) (OtherActor :type Actor%20Object%20Reference) (OtherComp :type Primitive%20Component%20Object%20Reference) (OtherBodyIndex :type Integer) (bFromSweep :type Boolean) (SweepResult :type Hit%20Result%20Structure%20%28by%20ref%29))
  ;[0.15 0.15 0.15 0.5] Enemy와 Player가 충돌한다면.. Player는 무조건 데미지를 입음
  (if (Components|ComponentHasTag OtherComp "PlayerDamageBody")
    (Class|BPIDamageable|TakeDamage(Message) OtherActor self (Math|Float|Truncate (.finalcontactdamage (Variables|Default|GetRuntimeStats))))))

(event Custom|CustomEvent
  (params (OtherActor :type Actor%20Object%20Reference)))

(event EventBeginPlay
  (|CallParentFunction))

(event EventTick
  (params (DeltaSeconds :type Float%20%28single-precision%29))
  (|CallParentFunction DeltaSeconds) ; 지금 이 노드는 비활성 상태입니다. \n핀을 끌어서 다른 노드를 연결하면 활성화됩니다.
)

(event Collision|EventActorBeginOverlap
  (params (OtherActor :type Actor%20Object%20Reference))
  (|CallParentFunction OtherActor))

(event EventGoDie
  (params (InKiller :type Actor%20Object%20Reference))
  (Variables|Default|SetExpSpawnLocationZ 5e+01)
  (Variables|Default|SetbIsDead true)
  ;[0.15 0.15 0.15 0.5] Die Anim 재생 딜레이 후, 다시 풀로 보내기
  (Utilities|FlowControl|Delay 0.5)
  (|CallParentFunction InKiller)
  (Default|RequestReturntoPool (Variables|Default|GetBPC_PoolableComponent))
  (Variables|Default|SetbIsDead false) ; 살아있는 상태의 애님을 재생하며 스폰시키기 위함
)

(event EventTakeDamage
  (params (AttackActor :type Actor%20Object%20Reference) (DamageAmount :type Integer))
  ;[0.15 0.15 0.15 0.5] 플레이어가 데미지를 줬다면 체력이 깎임
  (if (== AttackActor (Game|Player|GetPlayerPawn 0))
    (Variables|Default|SetCurHealth (- (Variables|Default|GetCurHealth) DamageAmount))
    (if (<= (Variables|Default|GetCurHealth) 0)
      (CallFunction|GoDie AttackActor))))

(fn ConstructionScript
  (|CallParentFunction))

(fn 새함수)