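; BP_SpawnSection is a box volume that marks an enemy spawn area and reacts to the player entering or leaving it.
; On BeginPlay it unhides the box and caches the first actor implementing BPI_CanManageEnemySpawn as the spawn manager.
; Player pawn overlap sends that manager the section as current through interface messages, and end overlap stops its spawn timer.
; Tick draws a debug box around the section every frame.
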(event OnComponentBeginOverlap(Section)
  (params (OverlappedComponent :type Primitive%20Component%20Object%20Reference) (OtherActor :type Actor%20Object%20Reference) (OtherComp :type Primitive%20Component%20Object%20Reference) (OtherBodyIndex :type Integer) (bFromSweep :type Boolean) (SweepResult :type Hit%20Result%20Structure%20%28by%20ref%29))
  (if (== OtherActor (Game|Player|GetPlayerPawn 0))
    (Class|BPICanManageEnemySpawn|SetCurSpawnSection(Message) (Variables|Default|GetEnemySpawnManager) self)))

(event OnComponentEndOverlap(Section)
  (params (OverlappedComponent :type Primitive%20Component%20Object%20Reference) (OtherActor :type Actor%20Object%20Reference) (OtherComp :type Primitive%20Component%20Object%20Reference) (OtherBodyIndex :type Integer))
  (if (== OtherActor (Game|Player|GetPlayerPawn 0))
    (Class|BPICanManageEnemySpawn|StopSpawnTimer(Message) (Variables|Default|GetEnemySpawnManager))))

(event EventBeginPlay
  (Development|SetHiddeninGame (Variables|Default|GetSection) false false)
  (bind _outactors (Actor|GetAllActorswithInterface "/Game/RuntimeSurvival/Core/Interface/BPI_CanManageEnemySpawn.BPI_CanManageEnemySpawn_C"))
  (Variables|Default|SetEnemySpawnManager (Utilities|Array|Get(acopy) _outactors)))

(event Collision|EventActorBeginOverlap
  (params (OtherActor :type Actor%20Object%20Reference)))

(event EventTick
  (params (DeltaSeconds :type Float%20%28single-precision%29))
  (bind _section (Variables|Default|GetSection))
  (Rendering|Debug|DrawDebugBox (Transformation|GetWorldLocation _section) (Components|Box|GetScaledBoxExtent _section) "(R=0.333333,G=0.085178,B=0.005415,A=1.000000)" (Transformation|GetWorldRotation _section) 0.0 2.0))

(fn ConstructionScript)