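; BP_Projectile_Bullet is a pooled bullet projectile for the player attack.
; Its pool activation and deactivation handlers toggle visibility, collision and ticking, so the actor can be reused, and print debug messages.
; On activation it also moves to the location of player pawn 0.
; The graph holds no movement or hit logic, as BeginPlay, Tick and overlap events are empty.
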(event EventBeginPlay)

(event Collision|EventActorBeginOverlap
  (params (OtherActor :type Actor%20Object%20Reference)))

(event EventTick
  (params (DeltaSeconds :type Float%20%28single-precision%29)))

(event EventHandlePoolDeactivated
  (Development|PrintString "Projectile 비활성화")
  (Rendering|SetActorHiddenInGame true)
  (Collision|SetActorEnableCollision false)
  (Actor|Tick|SetActorTickEnabled false))

(event EventHandlePoolActivated
  (Development|PrintString "Projectile 활성화")
  (Rendering|SetActorHiddenInGame false)
  (Collision|SetActorEnableCollision true)
  (Actor|Tick|SetActorTickEnabled true)
  (Transformation|SetActorLocation (Transformation|GetActorLocation (Game|Player|GetPlayerPawn 0)) false false))

(fn ConstructionScript)