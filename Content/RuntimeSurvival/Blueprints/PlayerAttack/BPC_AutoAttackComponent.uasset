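; Auto-attack actor component for player attacks, tracking owned attacks by ID, level and remaining spawn time.
; BeginPlay adds the default ProjectileBullet attack, ready to fire immediately, and starts a looping timer if auto-attack is enabled.
; UpdateAutoAttacks counts down each attack by the timer interval, resetting expired ones to a shared Cooldown, so Tick is unused.
; Triggering an attack currently only prints a message; nothing is spawned.
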(event EventBeginPlay
  ;[0.15 0.15 0.15 0.5] 기본 공격 세팅
  (Variables|Default|SetDefaultAutoAttackID "ProjectileBullet")
  (CallFunction|InitDefaultAttack)
  ;[0.15 0.15 0.15 0.5] AutoAttack 루프 돌리기
  (if (Variables|Default|GetbAutoAttackOnOff)
    (CallFunction|StartAutoAttackLoop)))

(event EventTick
  (params (DeltaSeconds :type Float%20%28single-precision%29)))

(fn AddAutoAttack
  (params (AutoAttackID :type Name))
  ;[0.15 0.15 0.15 0.5] 입력으로 들어온 AutoAttackID를 기반으로
  ; 남은 스폰 시간을 0으로 설정해  해당 공격을 얻자마자 바로 한 발 쏘도록 함, 그리고 공격 레벨은 1로 시작.
  (Utilities|Array|Add (Variables|Default|GetOwnedAutoAttacks) (Utilities|Struct|MakeST_OwnedAutoAttacks AutoAttackID 0.0 1)))

(fn InitDefaultAttack
  (CallFunction|AddAutoAttack (Variables|Default|GetDefaultAutoAttackID)))

(fn StartAutoAttackLoop
  (Utilities|Time|SetTimerbyEvent (EventDispatchers|CreateEvent :!event UpdateAutoAttacks) (Variables|Default|GetUpdateInterval) true))

(fn UpdateAutoAttacks
  (bind _ownedautoattacks (Variables|Default|GetOwnedAutoAttacks))
  (for _index (range 0 (- (Utilities|Array|Length (Variables|Default|GetOwnedAutoAttacks)) 1))
    (if (<= (- (.RemainSpawnTime (Utilities|Struct|BreakST_OwnedAutoAttacks (Utilities|Array|Get(acopy) _ownedautoattacks _index))) (Variables|Default|GetUpdateInterval)) 0.0)
      (LocalVariables|SetNextRemainSpawnTime (LocalVariables|GetCooldown))
      (Development|PrintString "AutoAttack 발동!" true true "(R=0.479167,G=0.072078,B=0.000000,A=1.000000)" 0.3)
      (else
        (LocalVariables|SetNextRemainSpawnTime (- (.RemainSpawnTime (Utilities|Struct|BreakST_OwnedAutoAttacks (Utilities|Array|Get(acopy) _ownedautoattacks _index))) (Variables|Default|GetUpdateInterval)))))
    (Utilities|Array|SetArrayElem _ownedautoattacks _index (Utilities|Struct|MakeST_OwnedAutoAttacks (.AutoAttackID (Utilities|Struct|BreakST_OwnedAutoAttacks (Utilities|Array|Get(acopy) _ownedautoattacks _index))) (LocalVariables|GetNextRemainSpawnTime) (.Level (Utilities|Struct|BreakST_OwnedAutoAttacks (Utilities|Array|Get(acopy) _ownedautoattacks _index)))))))