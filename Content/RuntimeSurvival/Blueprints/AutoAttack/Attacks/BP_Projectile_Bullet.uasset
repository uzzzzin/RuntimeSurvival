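; Pooled bullet projectile for the auto-attack system that fires at the nearest enemy within attack range.
; When an attack is prepared, it moves to the pool's spawn location and sphere-overlaps for enemies, setting a horizontal velocity toward the closest, or owner-forward if none overlap.
; On overlapping an enemy it records the hit, deals damage through the BPI_Damageable interface and requests return to the pool.
; A debug sphere shows the search range.
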(event OnComponentBeginOverlap(Collision)
  (params (OverlappedComponent :type Primitive%20Component%20Object%20Reference) (OtherActor :type Actor%20Object%20Reference) (OtherComp :type Primitive%20Component%20Object%20Reference) (OtherBodyIndex :type Integer) (bFromSweep :type Boolean) (SweepResult :type Hit%20Result%20Structure%20%28by%20ref%29))
  ;[0.15 0.15 0.15 0.5] Collision 충돌 시, 부모의 Hit Actors에 유효한 충돌 액터로 칠 액터를 집어 넣음, 사실은... 유효한 충돌 액터와 충돌하면 다시 풀로 돌아감(소멸)
  (if (Utilities|ClassIsChildOf (Utilities|GetClass OtherActor) (Variables|Default|GetValidCollisionActorClassType))
    (CallFunction|AddHitActors OtherActor)
    (if (Utilities|DoesObjectImplementInterface OtherActor "/Game/RuntimeSurvival/Core/Interface/BPI_Damageable.BPI_Damageable_C")
      (Class|BPIDamageable|TakeDamage(Message) OtherActor (Variables|Default|GetOwnerActor) (Math|Float|Truncate (Variables|Default|GetDamage)))
      (Default|RequestReturntoPool (Variables|Default|GetBPC_PoolableComponent)))))

(event EventBeginPlay
  (|CallParentFunction))

(event Collision|EventActorBeginOverlap
  (params (OtherActor :type Actor%20Object%20Reference))
  (|CallParentFunction OtherActor))

(event EventTick
  (params (DeltaSeconds :type Float%20%28single-precision%29))
  (|CallParentFunction DeltaSeconds))

(event EventPrepareAttack
  (params (InData :type ST%20Auto%20Attack%20Spawn%20Params%20Structure))
  ;[0.15 0.15 0.15 0.5] AutoAttackComponent에서 Pool Manager를 통해 HandlePoolActivated이 실행되고 난 후 실행됨.
  (CallFunction|AttackInitSetting InData))

(fn ConstructionScript)

(fn AttackInitSetting
  (params (InAutoAttackParams :type ST%20Auto%20Attack%20Spawn%20Params%20Structure))
  (|CallParentFunction InAutoAttackParams)
  (Variables|Default|SetProjectileMoveSpeed (.FinalProjectileMoveSpeed (Utilities|Struct|BreakST_AutoAttackSpawnParams InAutoAttackParams)))
  (Transformation|SetActorLocation (Variables|/Game/RuntimeSurvival/Blueprints/PoolSystem/BPC_PoolableComponent.BPC_PoolableComponent_C|GetInitLoc (Variables|Default|GetBPC_PoolableComponent)) false false)
  ;[0.15 0.15 0.15 0.5] 유효한 충돌로 칠 액터의 타입을 저장,
  ; Projectile 쏠 방향 지정
  (Variables|Default|SetValidCollisionActorClassType "/Game/RuntimeSurvival/Blueprints/Enemy/BP_Enemy_Base.BP_Enemy_Base_C")
  (CallFunction|FindDirfromTarget)
  (Rendering|Debug|DrawDebugSphere (Variables|/Game/RuntimeSurvival/Blueprints/PoolSystem/BPC_PoolableComponent.BPC_PoolableComponent_C|GetInitLoc (Variables|Default|GetBPC_PoolableComponent)) (Variables|Default|GetAttackRange) 12 "(R=1.000000,G=1.000000,B=1.000000,A=1.000000)" 1.0))

(fn FindDirfromTarget
  (bind _owneractor (Variables|Default|GetOwnerActor))
  (bind _returnvalue (Transformation|GetActorForwardVector _owneractor))
  ;[0.15 0.15 0.15 0.5] 초기값 세팅
  (LocalVariables|SetNearestDistance 1e+04)
  (LocalVariables|SetNearestEnemy 0)
  (Variables|Default|SetGoVelocity (* _returnvalue (Variables|Default|GetProjectileMoveSpeed)))
  (LocalVariables|SetStartDir _returnvalue)
  ;[0.15 0.15 0.15 0.5] Sphere Overlap 확인
  ; -> Overlap된 액터들 중 제일 가까이 있는 Enemy 액터를 구함
  ; -> 해당 액터를 향한 방향을 구하고 Projectile 속도 세팅하는데에 사용
  (bind (_outactors _returnvalue_2) (Collision|SphereOverlapActors (Variables|/Game/RuntimeSurvival/Blueprints/PoolSystem/BPC_PoolableComponent.BPC_PoolableComponent_C|GetInitLoc (Variables|Default|GetBPC_PoolableComponent)) (Variables|Default|GetAttackRange) (Utilities|Array|MakeArray "ObjectTypeQuery3") (Variables|Default|GetValidCollisionActorClassType)))
  (if _returnvalue_2
    (for _array_element _outactors
      (if (< (Transformation|GetDistanceTo _array_element) (LocalVariables|GetNearestDistance))
        (LocalVariables|SetNearestDistance (Transformation|GetDistanceTo _array_element))
        (LocalVariables|SetNearestEnemy _array_element)))
    (Utilities|IsValid (LocalVariables|GetNearestEnemy)
      (:Is%20Valid
        (Variables|Default|SetGoVelocity (* (Variables|Default|GetProjectileMoveSpeed) (Math|Vector|Normalize (- (Math|Vector|MakeVector (.x (Transformation|GetActorLocation (LocalVariables|GetNearestEnemy))) (.y (Transformation|GetActorLocation (LocalVariables|GetNearestEnemy))) (.z (Variables|/Game/RuntimeSurvival/Blueprints/PoolSystem/BPC_PoolableComponent.BPC_PoolableComponent_C|GetInitLoc (Variables|Default|GetBPC_PoolableComponent)))) (Variables|/Game/RuntimeSurvival/Blueprints/PoolSystem/BPC_PoolableComponent.BPC_PoolableComponent_C|GetInitLoc (Variables|Default|GetBPC_PoolableComponent))))))))
    (else
      (Development|PrintString "감지 범위 안에 적이 없습니다." true true "(R=0.625000,G=0.083672,B=0.000000,A=1.000000)")))
  (Variables|/Script/Engine.MovementComponent|SetVelocity (Variables|Default|GetProjectileMovement) (Variables|Default|GetGoVelocity)))

(fn AttackFinishSetting
  (|CallParentFunction))