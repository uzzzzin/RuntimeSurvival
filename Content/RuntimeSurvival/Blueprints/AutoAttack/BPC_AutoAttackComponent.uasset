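; Auto-attack component that holds its owner's attacks with level and remaining cooldown, starting with a default projectile bullet.
; A looping timer, rather than Tick, counts down cooldowns and executes attacks when due.
; Execution combines DataTable base values, per-level growth and owner stats into spawn params and the next cooldown.
; Attack actors come from an interface-discovered pool manager and receive those params through an interface message.
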(event EventBeginPlay
  ;[0.15 0.15 0.15 0.5] PoolManager 알기
  (CallFunction|InitPoolManager)
  ;[0.15 0.15 0.15 0.5] 기본 공격 세팅
  (Variables|Default|SetDefaultAutoAttackID "ProjectileBullet")
  (CallFunction|InitDefaultAttack)
  ;[0.15 0.15 0.15 0.5] AutoAttack 루프 돌리기
  (if (Variables|Default|GetbAutoAttackOnOff)
    (CallFunction|StartAutoAttackLoop)))

(event EventTick
  (params (DeltaSeconds :type Float%20%28single-precision%29)))

(fn AddAutoAttack
  (params (AutoAttackID :type Name))
  ;[0.15 0.15 0.15 0.5] 입력으로 들어온 AutoAttackID를 기반으로
  ; 남은 스폰 시간을 0으로 설정해  해당 공격을 얻자마자 바로 한 발 쏘도록 함, 그리고 공격 레벨은 1로 시작.
  (Utilities|Array|Add (Variables|Default|GetOwnedAutoAttacks) (Utilities|Struct|MakeST_OwnedAutoAttacks AutoAttackID 0.0 1)))

(fn InitDefaultAttack
  (CallFunction|AddAutoAttack (Variables|Default|GetDefaultAutoAttackID)))

(fn StartAutoAttackLoop
  ;[0.15 0.15 0.15 0.5] 자동공격 검사 주기(UpdateInterval) 마다
  ; AutoAttack의 남은 다음 스폰 시간을 계산하고 스폰을 처리하는 함수를 실행함
  (Utilities|Time|SetTimerbyEvent (EventDispatchers|CreateEvent :!event UpdateAutoAttacks) (Variables|Default|GetUpdateInterval) true))

(fn UpdateAutoAttacks
  (bind _ownedautoattacks (Variables|Default|GetOwnedAutoAttacks))
  ;[0.15 0.15 0.15 0.5] 컴포넌트가 들고 있는 AutoAttack들 Loop를 돌면서, 각 AutoAttack의 OwnedAutoAttack구조체에서 남은 다음 스폰 시간을 가져와 계산한다.
  ; 스폰할 타이밍이었다면 구조체 세팅하고 ExecuteAutoAttack으로 넘어감.
  ; 스폰할 시간이 아직 남아있다면, 해당 남은 스폰 시간만 계산하고 다시 구조체에 세팅함.
  (for _index (range 0 (- (Utilities|Array|Length (Variables|Default|GetOwnedAutoAttacks)) 1))
    (if (<= (- (.RemainSpawnTime (Utilities|Struct|BreakST_OwnedAutoAttacks (Utilities|Array|Get(acopy) _ownedautoattacks _index))) (Variables|Default|GetUpdateInterval)) 0.0)
      (Utilities|Array|SetArrayElem _ownedautoattacks _index (Utilities|Struct|MakeST_OwnedAutoAttacks (.AutoAttackID (Utilities|Struct|BreakST_OwnedAutoAttacks (Utilities|Array|Get(acopy) _ownedautoattacks _index))) (LocalVariables|GetNextRemainSpawnTime) (.Level (Utilities|Struct|BreakST_OwnedAutoAttacks (Utilities|Array|Get(acopy) _ownedautoattacks _index)))))
      ;[0.15 0.15 0.15 0.5] ExecuteAutoAttack()를 통해 계산된 CoolDown은
      ; AutoAttackComponent가 들고 있는 ST_OwnedAutoAttack의 멤버 Remain Spawn Time의 값을 갱신시킴.
      (bind (_finalcooldown _bsuccess) (CallFunction|ExecuteAutoAttack (Utilities|Struct|MakeST_OwnedAutoAttacks (.AutoAttackID (Utilities|Struct|BreakST_OwnedAutoAttacks (Utilities|Array|Get(acopy) _ownedautoattacks _index))) (LocalVariables|GetNextRemainSpawnTime) (.Level (Utilities|Struct|BreakST_OwnedAutoAttacks (Utilities|Array|Get(acopy) _ownedautoattacks _index))))))
      (if _bsuccess
        (Utilities|Array|SetArrayElem _ownedautoattacks _index (Utilities|Struct|MakeST_OwnedAutoAttacks (.AutoAttackID (Utilities|Struct|BreakST_OwnedAutoAttacks (Utilities|Array|Get(acopy) _ownedautoattacks _index))) _finalcooldown (.Level (Utilities|Struct|BreakST_OwnedAutoAttacks (Utilities|Array|Get(acopy) _ownedautoattacks _index))))))
      (else
        (LocalVariables|SetNextRemainSpawnTime (- (.RemainSpawnTime (Utilities|Struct|BreakST_OwnedAutoAttacks (Utilities|Array|Get(acopy) _ownedautoattacks _index))) (Variables|Default|GetUpdateInterval)))
        (Utilities|Array|SetArrayElem _ownedautoattacks _index (Utilities|Struct|MakeST_OwnedAutoAttacks (.AutoAttackID (Utilities|Struct|BreakST_OwnedAutoAttacks (Utilities|Array|Get(acopy) _ownedautoattacks _index))) (LocalVariables|GetNextRemainSpawnTime) (.Level (Utilities|Struct|BreakST_OwnedAutoAttacks (Utilities|Array|Get(acopy) _ownedautoattacks _index)))))))))

(fn ExecuteAutoAttack
  (params (InWillSpawnOwnedAutoAttacks :type ST%20Owned%20Auto%20Attacks%20Structure))
  (LocalVariables|SetCurAttackLevelOffset (- (.level InWillSpawnOwnedAutoAttacks) 1))
  ;[0.15 0.15 0.15 0.5] 해당 AutoAttack의 OriginData를 가져옴
  (bind (_bfound _outautoattackorigindata) (CallFunction|GetAutoAttackOriginData (.autoattackid InWillSpawnOwnedAutoAttacks)))
  ;[0.15 0.15 0.15 0.5] AutoAttack의 OriginData에 있는 Base와 Player의 스탯과 레벨별 조절값을 통해,
  ; 최종적으로 AutaAttack에게 보내는 ST_AutoAttackSpawnParams 구조체를 만듦.
  (if _bfound
    (bind _outattackstats (Class|BPICanProvidePlayerStat|GetAttackStats(Message) (Components|GetOwner)))
    ;[0.15 0.15 0.15 0.5] 이번에 발사해야 할 자동 공격의 개수를 가져와
    ; PoolManager에게 그만큼의 횟수만큼 해당 AutoAttackClassType의 객체를 풀에서 가져오도록 요청함.
    (for _index (range 0 (- (Math|Integer|Max(Integer) (+ (.projectilecountbonus _outattackstats) (.BaseProjectileCount (Utilities|Struct|BreakST_AutoAttackData _outautoattackorigindata)) (/ (LocalVariables|GetCurAttackLevelOffset) (.ProejectileCountBounsInterval (Utilities|Struct|BreakST_AutoAttackData _outautoattackorigindata)))) 1) 1))
      (bind _outactor (Class|BPICanManageObjectPool|GetActorinPoolInterface(Message) (Variables|Default|GetPoolManager) (.AutoAttackClass (Utilities|Struct|BreakST_AutoAttackData _outautoattackorigindata)) (Transformation|GetActorLocation (Components|GetOwner))))
      (Class|BPIAutoAttackActor|PrepareAttack(Message) _outactor (Utilities|Struct|MakeST_AutoAttackSpawnParams (Components|GetOwner) (* (.damagemultiplier _outattackstats) (.BaseDamage (Utilities|Struct|BreakST_AutoAttackData _outautoattackorigindata)) (+ (* (LocalVariables|GetCurAttackLevelOffset) (.DamageGrowthPerLevel (Utilities|Struct|BreakST_AutoAttackData _outautoattackorigindata))) 1.0)) (* (.BaseLifeTime (Utilities|Struct|BreakST_AutoAttackData _outautoattackorigindata)) (+ (* (LocalVariables|GetCurAttackLevelOffset) (.LifeTimeGrowthPerLevel (Utilities|Struct|BreakST_AutoAttackData _outautoattackorigindata))) 1.0)) (* (.attackrangemultiplier _outattackstats) (.BaseAttackRange (Utilities|Struct|BreakST_AutoAttackData _outautoattackorigindata)) (+ (* (LocalVariables|GetCurAttackLevelOffset) (.AttackRangeGrowthPerLevel (Utilities|Struct|BreakST_AutoAttackData _outautoattackorigindata))) 1.0)) (* (.projectilespeedmultiplier _outattackstats) (.BaseProjectileMoveSpeed (Utilities|Struct|BreakST_AutoAttackData _outautoattackorigindata)) (+ (* (LocalVariables|GetCurAttackLevelOffset) (.ProjectileSpeedGrowthPerLevel (Utilities|Struct|BreakST_AutoAttackData _outautoattackorigindata))) 1.0)) (* (.arearaiusmultiplier _outattackstats) (.BaseAreaRadius (Utilities|Struct|BreakST_AutoAttackData _outautoattackorigindata)) (+ (* (LocalVariables|GetCurAttackLevelOffset) (.AreaRadiusGrowthPerLevel (Utilities|Struct|BreakST_AutoAttackData _outautoattackorigindata))) 1.0)) (.level InWillSpawnOwnedAutoAttacks)))
      (return (/ (* (.BaseCoolDown (Utilities|Struct|BreakST_AutoAttackData _outautoattackorigindata)) (Math|Float|Max(Float) (- 1.0 (* (LocalVariables|GetCurAttackLevelOffset) (.CooldownReduceperLevel (Utilities|Struct|BreakST_AutoAttackData _outautoattackorigindata)))) (.MinCooldownMultiplier (Utilities|Struct|BreakST_AutoAttackData _outautoattackorigindata)))) (.attackspeedmultiplier _outattackstats)) (Utilities|IsValid _outactor)))
    (else
      (Development|PrintString "AutoAttack 없어!" true true "(R=1.000000,G=0.117985,B=0.000000,A=1.000000)"))))

(fn GetAutoAttackOriginData
  (params (AutoAttackID :type Name))
  (bind _returnvalue (Utilities|GetDataTableRow (Variables|Default|GetAutoAttackOriginData) AutoAttackID)
    (:then
      (return true _returnvalue))
    (:RowNotFound
      (return false ""))))

(fn InitPoolManager
  ;[0.15 0.15 0.15 0.5] PoolManager만이 CanManageObjectPool 인터페이스를 가지고,
  ; PoolManager는 오로지 하나이기 때문에 배열의 0번째로 가져와도 됨.
  (bind _outactors (Actor|GetAllActorswithInterface "/Game/RuntimeSurvival/Core/Interface/BPI_CanManageObjectPool.BPI_CanManageObjectPool_C"))
  (if (Utilities|Array|IsNotEmpty _outactors)
    (Variables|Default|SetPoolManager (Utilities|Array|Get(acopy) _outactors))))