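; BP_AutoAttackBase is a pooled base actor for auto attacks, with an empty damage function and default-value animation getters.
; AttackInitSetting copies owner, damage, range and level from the params, then starts a short fixed lifetime timer meant to return it to the pool via BPCPoolableComponent.
; BPI_Poolable events toggle visibility, collision and tick, and deactivation clears the recorded hit actors and valid collision class.
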(event Custom|AddHitActors
  (params (InHitActor :type Actor%20Object%20Reference))
  (Utilities|Array|Add (Variables|Default|GetHitActors) InHitActor))

(event Custom|OnLifetimeExpired
  ;[0.15 0.15 0.15 0.5] OnLifetimeExpired :: Lifetime이 끝났으니 다시 풀로..
  (Default|RequestReturntoPool (Variables|Default|GetBPC_PoolableComponent)))

(event EventHandlePoolActivated
  (params (InLocation :type Vector :default "0, 0, 0"))
  ;[0.15 0.15 0.15 0.5] BPI_Poolable :: HandlePoolActivated
  (Variables|/Game/RuntimeSurvival/Blueprints/PoolSystem/BPC_PoolableComponent.BPC_PoolableComponent_C|SetInitLoc (Variables|Default|GetBPC_PoolableComponent) InLocation)
  (Rendering|SetActorHiddenInGame false)
  (Collision|SetActorEnableCollision true)
  (Actor|Tick|SetActorTickEnabled true))

(event EventHandlePoolDeactivated
  ;[0.15 0.15 0.15 0.5] BPI_Poolable :: HandlePoolDeactivated
  (Rendering|SetActorHiddenInGame true)
  (Collision|SetActorEnableCollision false)
  (Actor|Tick|SetActorTickEnabled false)
  (CallFunction|AttackFinishSetting))

(fn ConstructionScript)

(fn AttackInitSetting
  (params (InAutoAttackParams :type ST%20Auto%20Attack%20Spawn%20Params%20Structure))
  (bind (_onweractor _finaldamage _finallifetime _finalattackrange _finalprojectilemovespeed _finalarearadius _attacklevel) (Utilities|Struct|BreakST_AutoAttackSpawnParams InAutoAttackParams))
  (Variables|Default|SetOwnerActor _onweractor)
  (Variables|Default|SetDamage _finaldamage)
  (Variables|Default|SetLifeTime 1.0)
  (Variables|Default|SetAttackRange _finalattackrange)
  (Variables|Default|SetAttackLevel _attacklevel)
  ;[0.15 0.15 0.15 0.5] LifeTime이 다 된다면 OnLifetimeExpired로...
  (Utilities|Time|SetTimerbyEvent (EventDispatchers|CreateEvent :!event Custom|OnLifetimeExpired) (Variables|Default|GetLifeTime)))

(fn AttackFinishSetting
  (Variables|Default|SetValidCollisionActorClassType 0)
  (Utilities|Array|Clear (Variables|Default|GetHitActors)))

(fn ApplyDamagetoTarget)

(fn IsinAirforAnim
  (return false))

(fn GetZSpeedforAnim
  (return 0.0))

(fn GetMoveSpeedforAnim
  (return 0.0))