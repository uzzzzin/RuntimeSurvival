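; Player character for a runtime survival game, handling Enhanced Input camera-relative movement, clamped-pitch look and jumping.
; BPCStatComponent holds stats, exposed through getters and changed by experience pickups, heals and bonuses; its level-up event is bound for BPCPlayerInventory handling.
; Enemy hits subtract multiplier-scaled damage from health, triggering death and stopping movement at zero.
; Interface events gate movement, including a timed pause on landing, and getters supply animation state.
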(event Input|EnhancedActionEvents|EnhancedInputActionIA_Jump
  (params (ActionValue :type Boolean) (ElapsedSeconds :type Float%20%28double-precision%29) (TriggeredSeconds :type Float%20%28double-precision%29) (InputAction :type Input%20Action%20Object%20Reference :default "/Game/RuntimeSurvival/Core/Input/IA_Jump.IA_Jump"))
  ;[0.15 0.15 0.15 0.5] IA_Jump : 점프
  (:Triggered
    (Character|Jump))
  (:Completed
    (Character|StopJumping)))

(event Input|EnhancedActionEvents|EnhancedInputActionIA_Look
  (params (ActionValue :type Vector%202D%20Structure) (ElapsedSeconds :type Float%20%28double-precision%29) (TriggeredSeconds :type Float%20%28double-precision%29) (InputAction :type Input%20Action%20Object%20Reference :default "/Game/RuntimeSurvival/Core/Input/IA_Look.IA_Look"))
  (bind (_x _y) (Math|Vector2D|BreakVector2D ActionValue))
  (bind _mousesensitivity (Variables|Default|GetMouseSensitivity))
  ;[0.15 0.15 0.15 0.5] IA_Look : 마우스 Look 입력을 받아 Controller의 Rotation을 갱신, Pitch는 Clamp를 통해 위/아래 회전을 제한함.
  (Variables|Default|SetCurrentMouseRotate (Pawn|GetControlRotation :!class /Script/Engine.Pawn))
  (Pawn|SetControlRotation (Game|GetPlayerController 0) (Math|Rotator|MakeRotator 0.0 (Math|Float|Clamp(Float) (+ (.pitch (Variables|Default|GetCurrentMouseRotate)) (* _mousesensitivity _y)) (Variables|Default|GetCameraPitchMin) (Variables|Default|GetCameraPitchMax)) (+ (* _x _mousesensitivity) (.yaw (Variables|Default|GetCurrentMouseRotate))))))

(event Input|EnhancedActionEvents|EnhancedInputActionIA_Movement
  (params (ActionValue :type Vector%202D%20Structure) (ElapsedSeconds :type Float%20%28double-precision%29) (TriggeredSeconds :type Float%20%28double-precision%29) (InputAction :type Input%20Action%20Object%20Reference :default "/Game/RuntimeSurvival/Core/Input/IA_Movement.IA_Movement"))
  (bind (_x _y) (Math|Vector2D|BreakVector2D ActionValue))
  (bind _returnvalue (Pawn|GetControlRotation :!class /Script/Engine.Pawn))
  (bind _returnvalue_2 (Math|Rotator|MakeRotator 0.0 0.0 (.yaw _returnvalue)))
  (bind _returnvalue_3 (Math|Vector|GetForwardVector _returnvalue_2))
  (bind _returnvalue_4 (Math|Vector|GetRightVector _returnvalue_2))
  (bind _returnvalue_5 (* _y _returnvalue_3))
  (bind _returnvalue_6 (* _returnvalue_4 _x))
  (bind _returnvalue_7 (+ _returnvalue_5 _returnvalue_6))
  ;[0.15 0.15 0.15 0.5] IA_Movement : 카메라 회전 Yaw를 기준으로 플레이어 이동.
  ; Yaw를 추출해 이동의 기준이 될 방향을 만들고, Right/Forward에 적용함. (카메라 Pitch는 이동 계산에서 제외!)
  (if (Variables|Default|GetbCanMove)
    (Pawn|Input|AddMovementInput _returnvalue_3 _y false)
    (Pawn|Input|AddMovementInput _returnvalue_4 _x false)
    ;[0.15 0.15 0.15 0.5] 이동 입력이 있을 시에만, LastMoveDirection 세팅
    (if (> (Math|Vector|VectorLength _returnvalue_7) 0.05)
      (Variables|Default|SetLastMoveDirection (Math|Vector|Normalize _returnvalue_7)))))

(event EventBeginPlay
  ;[0.15 0.15 0.15 0.5] IMC 등록
  (Input|AddMappingContext (PlayerController|LocalPlayerSubsystems|GetEnhancedInputLocalPlayerSubsystem) "/Game/RuntimeSurvival/Core/Input/IMC_Player.IMC_Player" 0 "(bIgnoreAllPressedKeysUntilRelease=True,bForceImmediately=False,bNotifyUserSettings=False)")
  (EventDispatchers|BindEventtoOnPlayerLevelUp (Variables|Default|GetBPC_StatComponent) (EventDispatchers|CreateEvent :!event HandlePlayerLevelUp)))

(event EventAddMaxHPbyPercentInterface
  (params (InAddPercent :type Float%20%28double-precision%29))
  (Default|AddMaxHPbyPercent (Variables|Default|GetBPC_StatComponent) InAddPercent))

(event EventOnLanded
  (params (Hit :type Hit%20Result%20Structure%20%28by%20ref%29))
  ;[0.15 0.15 0.15 0.5] Event_OnLanded : 착지할 때, 잠시 이동을 멈추고 다시 이동을 활성화
  (CallFunction|StopMovement)
  (Utilities|Time|SetTimerbyEvent (EventDispatchers|CreateEvent :!event ResumeMovement) (Variables|Default|GetMoveStopDuration)))

(event EventResumeMovement
  ;[0.15 0.15 0.15 0.5] BPI_CanManageInputMovement :: ResumeMovement
  (Variables|Default|SetbCanMove true))

(event EventStopMovement
  ;[0.15 0.15 0.15 0.5] BPI_CanManageInputMovement :: StopMovement
  (Variables|Default|SetbCanMove false))

(event EventTick
  (params (DeltaSeconds :type Float%20%28single-precision%29)))

(event EventExp
  (params (InExp :type Integer))
  ;[0.15 0.15 0.15 0.5] Enemy를 죽여 스폰된 Exp를 주웠어요
  (Default|AddExp (Variables|Default|GetBPC_StatComponent) InExp))

(event EventTakeDamage
  (params (AttackActor :type Actor%20Object%20Reference) (DamageAmount :type Integer))
  (bind _bisenemy (Class|BPIIsEnemy|IsEnemy(Message) AttackActor))
  (if _bisenemy
    ;[0.15 0.15 0.15 0.5] 적과 부딪히면, 적의 데미지에 데미지 받는 스탯을 계산해 현재 체력을 깎음.
    (bind _output_get (Variables|/Game/RuntimeSurvival/Blueprints/Player/BPC_PlayerStatComponent.BPC_PlayerStatComponent_C|SetVitalStats (Variables|Default|GetBPC_StatComponent) (Utilities|Struct|MakeST_PlayerVitalStat (.maxhealth (Variables|/Game/RuntimeSurvival/Blueprints/Player/BPC_PlayerStatComponent.BPC_PlayerStatComponent_C|GetVitalStats (Variables|Default|GetBPC_StatComponent))) (- (.curhealth (Variables|/Game/RuntimeSurvival/Blueprints/Player/BPC_PlayerStatComponent.BPC_PlayerStatComponent_C|GetVitalStats (Variables|Default|GetBPC_StatComponent))) (* DamageAmount (.damagetakenmultiplier (Variables|/Game/RuntimeSurvival/Blueprints/Player/BPC_PlayerStatComponent.BPC_PlayerStatComponent_C|GetVitalStats (Variables|Default|GetBPC_StatComponent))))) (.healregenpersecondmultiplier (Variables|/Game/RuntimeSurvival/Blueprints/Player/BPC_PlayerStatComponent.BPC_PlayerStatComponent_C|GetVitalStats (Variables|Default|GetBPC_StatComponent))) (.damagetakenmultiplier (Variables|/Game/RuntimeSurvival/Blueprints/Player/BPC_PlayerStatComponent.BPC_PlayerStatComponent_C|GetVitalStats (Variables|Default|GetBPC_StatComponent))))))
    (if (<= (.curhealth _output_get) 0)
      (CallFunction|GoDie))))

(event EventHealbyMaxHealthPercentInterface
  (params (InPercent :type Float%20%28double-precision%29))
  (Default|HealbyMaxHealthPercent (Variables|Default|GetBPC_StatComponent) InPercent))

(event EventGoDie
  ;[0.15 0.15 0.15 0.5] BPI_Damageable::GoDie
  (Variables|Default|SetbDead true)
  (CallFunction|StopMovement))

(event EventAddMoveSpeedInterface
  (params (InBonusMoveSpeed :type Float%20%28double-precision%29))
  (bind _charactermovement (Variables|Character|GetCharacterMovement))
  (bind _outmovespeed (Default|AddMoveSpeed (Variables|Default|GetBPC_StatComponent) InBonusMoveSpeed))
  (Variables|/Script/Engine.CharacterMovementComponent|SetMaxWalkSpeed _charactermovement (* _outmovespeed (Variables|/Script/Engine.CharacterMovementComponent|GetMaxWalkSpeed _charactermovement))))

(fn ConstructionScript)

(fn HandlePlayerLevelUp
  (params (InCurLevel :type Integer))
  (Default|HandlePlayerLevelUp (Variables|Default|GetBPC_PlayerInventory) InCurLevel))

(fn GetAttackStats
  (return (Variables|/Game/RuntimeSurvival/Blueprints/Player/BPC_PlayerStatComponent.BPC_PlayerStatComponent_C|GetAttackStats (Variables|Default|GetBPC_StatComponent))))

(fn GetMovementStats
  (return (Variables|/Game/RuntimeSurvival/Blueprints/Player/BPC_PlayerStatComponent.BPC_PlayerStatComponent_C|GetMovementStats (Variables|Default|GetBPC_StatComponent))))

(fn GetMoveSpeedforAnim
  (return (Math|Vector|VectorLengthXY (Transformation|GetVelocity))))

(fn GetUtilStats
  (return (Variables|/Game/RuntimeSurvival/Blueprints/Player/BPC_PlayerStatComponent.BPC_PlayerStatComponent_C|GetUtilStats (Variables|Default|GetBPC_StatComponent))))

(fn GetVitalStats
  (return (Variables|/Game/RuntimeSurvival/Blueprints/Player/BPC_PlayerStatComponent.BPC_PlayerStatComponent_C|GetVitalStats (Variables|Default|GetBPC_StatComponent))))

(fn GetZSpeedforAnim
  (return (.z (Transformation|GetVelocity))))

(fn IsDead
  (return (Variables|Default|GetbDead)))

(fn IsinAirforAnim
  (return (AI|Components|NavMovement|IsFalling (Variables|Character|GetCharacterMovement))))