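; BPC_PlayerStatComponent is a player component that holds the character's stats, grouped into attack, movement, utility and vital sets.
; Each group is exposed through its own getter, which returns the stored variable unchanged.
; It has no runtime logic of its own, as BeginPlay and Tick are empty, disabled placeholder events.
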(event EventBeginPlay)

(event EventTick
  (params (DeltaSeconds :type Float%20%28single-precision%29)))

(fn GetAttackStats
  (return (Variables|Default|GetAttackStats)))

(fn GetMovementStats
  (return (Variables|Default|GetMovementStats)))

(fn GetUtilStats
  (return (Variables|Default|GetUtilStats)))

(fn GetVitalStats
  (return (Variables|Default|GetVitalStats)))