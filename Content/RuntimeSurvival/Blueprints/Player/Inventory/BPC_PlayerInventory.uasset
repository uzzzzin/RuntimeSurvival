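; Player inventory component that creates, stores and removes item objects for its owner.
; Adding an item looks up its data table row by ID, constructs that row's class, initializes it and fires its pickup callback, storing it only if flagged KeepInInventory.
; Items request their own removal through a bound dispatcher, while HandleItemRemove notifies and drops the matching entry.
; Player level-ups are forwarded to every stored item.
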(event EventBeginPlay)

(event EventTick
  (params (DeltaSeconds :type Float%20%28single-precision%29)))

(fn AddItemtoArray
  (params (InItemID :type Name))
  (bind _outitemdata (Class|BPICanProvideGameData|GetItemData(Message) (Game|GetGameInstance)))
  (bind _returnvalue (Utilities|GetDataTableRow _outitemdata InItemID)
    (:then
      (Development|PrintString "찾았어요 아이템")
      ;[0.15 0.15 0.15 0.5] 아이템 실질적 옵젝 생성 및 초기화 세팅
      (bind _returnvalue_2 (Game|ConstructObjectfromClass (.ItemClassType (Utilities|Struct|BreakST_Normal_Item _returnvalue))))
      (Default|InitItem _returnvalue_2 (Components|GetOwner) InItemID)
      ;[0.15 0.15 0.15 0.5] 아이템의 디스패쳐에 바인딩.. 구독, 이벤트 연결
      (EventDispatchers|BindEventtoOnRequestRemoveSelffromInventory _returnvalue_2 (EventDispatchers|CreateEvent :!event HandleItemRemove))
      (if (.bKeepInInventory (Utilities|Struct|BreakST_Normal_Item _returnvalue))
        (Utilities|Array|Add (Variables|Default|GetOwnedItems) (Utilities|Struct|MakeST_OwnedItem InItemID _returnvalue_2)))
      (Default|OnPickedUp _returnvalue_2)
      (return))))

(fn HandleItemRemove
  (params (InItemInstance :type BP%20Item%20Base%20Object%20Reference))
  ;[0.15 0.15 0.15 0.5] 아이템 배열을 순회하며 지우려고 요청 들어온 아이템을 찾아 배열에서 뺀다
  (bind (_array_element _array_index) (Utilities|Array|ForEachLoopwithBreak (Variables|Default|GetOwnedItems) :!label _label)
    (:LoopBody
      (if (== (.iteminstance _array_element) InItemInstance)
        (Default|OnRemoved InItemInstance)
        (Utilities|Array|RemoveIndex (Variables|Default|GetOwnedItems) _array_index)
        (goto _label Break)))))

(fn HandlePlayerLevelUp
  (params (InNewLevel :type Integer))
  (for _array_element (Variables|Default|GetOwnedItems)
    (Default|OnPlayerLevelUp (.iteminstance _array_element) InNewLevel)))