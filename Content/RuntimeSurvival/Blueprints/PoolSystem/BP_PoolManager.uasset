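; Object pool manager that pre-spawns and recycles actors per class for the runtime survival game.
; BeginPlay fills each PoolDataList entry's waiting array to its initial size and registers itself with each actor's BPC_PoolableComponent.
; Getting pops the last waiting actor and activates it through BPI_Poolable, only printing a warning when empty.
; Returning moves the actor to PoolActorsLocation, deactivates it and requeues it, with an InPool flag blocking double returns.
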(event EventBeginPlay
  (bind _tempactorarr (Variables|Default|GetTempActorArr))
  ;[0.15 0.15 0.15 0.5] PoolDataList를 순회하며, TempActorArr에 Pooled Actor Class 타입의 객체를 Initial Pool Size 개수만큼 스폰해 TempActorArray에 담아두고,
  ; 해당 객체들의 스폰이 끝났을 때 WaitingActorArray를 TempActorArray의 값들로 갈아끼운다.
  ; 그리고 스폰할 때, 미리 ReturnActorToPool 시켜둠!
  (for _index (range (Variables|Default|GetCurPoolDataListIdx) (- (Utilities|Array|Length (Variables|Default|GetPoolDataList)) 1))
    (Utilities|Array|Clear (Variables|Default|GetTempActorArr))
    (for _index_2 (range 0 (- (.InitialPoolSize (Utilities|Struct|BreakST_ObjectpoolData (Utilities|Array|Get(acopy) (Variables|Default|GetPoolDataList) _index))) 1))
      (bind _returnvalue (Game|SpawnActorfromClass (.PooledActorClass (Utilities|Struct|BreakST_ObjectpoolData (Utilities|Array|Get(acopy) (Variables|Default|GetPoolDataList) _index))) (Math|Conversions|ToTransform(Vector) (Math|Vector|MakeVector 0.0 0.0 0.0)) "AlwaysSpawn" "MultiplyWithRoot" 0 0))
      (Utilities|Array|Add _tempactorarr _returnvalue)
      (CallFunction|ReturnActortoPool _returnvalue)
      (Utilities|IsValid (Actor|GetComponentbyClass _returnvalue "/Game/RuntimeSurvival/Blueprints/PoolSystem/BPC_PoolableComponent.BPC_PoolableComponent_C")
        (:Is%20Valid
          (Default|SetPoolManager (Actor|GetComponentbyClass _returnvalue "/Game/RuntimeSurvival/Blueprints/PoolSystem/BPC_PoolableComponent.BPC_PoolableComponent_C") self))))
    (Utilities|Array|SetArrayElem (Variables|Default|GetPoolDataList) (Variables|Default|GetCurPoolDataListIdx) (Utilities|Struct|MakeST_ObjectpoolData (.PooledActorClass (Utilities|Struct|BreakST_ObjectpoolData (Utilities|Array|Get(acopy) (Variables|Default|GetPoolDataList) _index))) (.InitialPoolSize (Utilities|Struct|BreakST_ObjectpoolData (Utilities|Array|Get(acopy) (Variables|Default|GetPoolDataList) _index))) _tempactorarr))
    (Math|Integer|IncrementInt (Variables|Default|GetCurPoolDataListIdx))))

(event Collision|EventActorBeginOverlap
  (params (OtherActor :type Actor%20Object%20Reference)))

(event EventTick
  (params (DeltaSeconds :type Float%20%28single-precision%29)))

(event EventReturnActortoPoolInterface
  (params (InActor :type Actor%20Object%20Reference))
  (CallFunction|ReturnActortoPool InActor))

(fn ConstructionScript)

(fn GetActorinPool
  (params (InActorClassType :type Actor%20Class%20Reference) (InActorLocation :type Vector))
  (LocalVariables|SetInClassType InActorClassType)
  ;[0.15 0.15 0.15 0.5] 인자로 들어온 ClassType에 해당하는 PoolDataList Array의 Index를 찾는 과정
  (bind (_array_element _array_index) (Utilities|Array|ForEachLoopwithBreak (Variables|Default|GetPoolDataList) :!label _label)
    (:LoopBody
      (if (== (LocalVariables|GetInClassType) (.PooledActorClass (Utilities|Struct|BreakST_ObjectpoolData _array_element)))
        (LocalVariables|SetFoundIdx _array_index)
        (goto _label Break)))
    (:Completed
      (if (> (Utilities|Array|Length (.waitingactorarray (Utilities|Array|Get(acopy) (Variables|Default|GetPoolDataList) (LocalVariables|GetFoundIdx)))) 0)
        ;[0.15 0.15 0.15 0.5] 인자로 들어온 ClassType에 해당하는 ST_ObejctPoolData의 WaitingActorVector에서 제일 끝에 있는 액터를 WaitingActorVector에서 제거하고 가져온다
        (LocalVariables|SetPopActorInPool (Utilities|Array|Get(acopy) (.waitingactorarray (Utilities|Array|Get(acopy) (Variables|Default|GetPoolDataList) (LocalVariables|GetFoundIdx))) (- (Utilities|Array|Length (.waitingactorarray (Utilities|Array|Get(acopy) (Variables|Default|GetPoolDataList) (LocalVariables|GetFoundIdx)))) 1)))
        (Utilities|Array|RemoveIndex (.waitingactorarray (Utilities|Array|Get(acopy) (Variables|Default|GetPoolDataList) (LocalVariables|GetFoundIdx))) (- (Utilities|Array|Length (.waitingactorarray (Utilities|Array|Get(acopy) (Variables|Default|GetPoolDataList) (LocalVariables|GetFoundIdx)))) 1))
        (Utilities|Array|SetArrayElem (Variables|Default|GetPoolDataList) (Variables|Default|GetCurPoolDataListIdx) (Utilities|Struct|MakeST_ObjectpoolData (.pooledactorclass (Utilities|Array|Get(acopy) (Variables|Default|GetPoolDataList) (LocalVariables|GetFoundIdx))) (.initialpoolsize (Utilities|Array|Get(acopy) (Variables|Default|GetPoolDataList) (LocalVariables|GetFoundIdx))) (.waitingactorarray (Utilities|Array|Get(acopy) (Variables|Default|GetPoolDataList) (LocalVariables|GetFoundIdx)))))
        ;[0.15 0.15 0.15 0.5] Pop해온 액터가 풀 될 때 스스로 내부에서 해야 할 것들을 진행하는 인터페이스 함수를 실행한다.
        (Class|BPIPoolable|HandlePoolActivated(Message) (LocalVariables|GetPopActorInPool) InActorLocation)
        ;[0.15 0.15 0.15 0.5] 새로 풀에서 빼왔으니, 풀에 없음 처리
        (Variables|/Game/RuntimeSurvival/Blueprints/PoolSystem/BPC_PoolableComponent.BPC_PoolableComponent_C|SetbInPool (Actor|GetComponentbyClass (LocalVariables|GetPopActorInPool) "/Game/RuntimeSurvival/Blueprints/PoolSystem/BPC_PoolableComponent.BPC_PoolableComponent_C") false)
        (return (LocalVariables|GetPopActorInPool))
        (else
          (Development|PrintString "풀에서 가져올 액터가 없어요! 준비된 액터 수량 부족!" true true "(R=0.677083,G=0.090623,B=0.000000,A=1.000000)"))))))

(fn ReturnActortoPool
  (params (InActor :type Actor%20Object%20Reference))
  ;[0.15 0.15 0.15 0.5] 풀 요청 들어온 액터가 풀 매니저가 관리하는 타입인지 확인
  (if (Utilities|DoesObjectImplementInterface InActor "/Game/RuntimeSurvival/Core/Interface/BPI_Poolable.BPI_Poolable_C")
    ;[0.15 0.15 0.15 0.5] 해당 객체가 풀에 있지 않을 때만 풀에 넣음
    (if (not (Variables|/Game/RuntimeSurvival/Blueprints/PoolSystem/BPC_PoolableComponent.BPC_PoolableComponent_C|GetbInPool (Actor|GetComponentbyClass InActor "/Game/RuntimeSurvival/Blueprints/PoolSystem/BPC_PoolableComponent.BPC_PoolableComponent_C")))
      ;[0.15 0.15 0.15 0.5] 다시 풀로 들어오기 위해, 풀 지정 자리 (PoolActorsLocation)에 위치를 세팅하고
      ; 인자로 들어온 액터가 비활성화 될 때 처리해야 할 것들이 담긴 인터페이스 함수를 실행한다
      (Utilities|IsValid InActor
        (:Is%20Valid
          (Transformation|SetActorLocation InActor (Variables|Default|GetPoolActorsLocation) false false)
          (Class|BPIPoolable|HandlePoolDeactivated(Message) InActor)
          (Utilities|Array|Clear (Variables|Default|GetTempActorArr))
          ;[0.15 0.15 0.15 0.5] 인자로 들어온 액터의 ClassType에 해당하는 PoolDataList 배열의 인덱스를 찾아 저장
          (bind (_array_element _array_index) (Utilities|Array|ForEachLoopwithBreak (Variables|Default|GetPoolDataList) :!label _label)
            (:LoopBody
              (if (== (.PooledActorClass (Utilities|Struct|BreakST_ObjectpoolData _array_element)) (Utilities|GetClass InActor))
                (goto _label Break)))
            (:Completed
              (LocalVariables|SetFoundIdx _array_index)
              (bind _output_get (Variables|Default|SetTempActorArr (.WaitingActorArray (Utilities|Struct|BreakST_ObjectpoolData _array_element))))
              ;[0.15 0.15 0.15 0.5] 찾은 인덱스에 해당하는 ST_ObjectPooData의 WaitingArray에
              ; 인자로 들어온 액터를 추가하고 다시 PoolDataList 배열의 구조체 값을 저장한다
              (Utilities|Array|Add _output_get InActor)
              (Utilities|Array|SetArrayElem (Variables|Default|GetPoolDataList) (LocalVariables|GetFoundIdx) (Utilities|Struct|MakeST_ObjectpoolData (.PooledActorClass (Utilities|Struct|BreakST_ObjectpoolData _array_element)) (.InitialPoolSize (Utilities|Struct|BreakST_ObjectpoolData _array_element)) (Variables|Default|GetTempActorArr)))
              (Variables|/Game/RuntimeSurvival/Blueprints/PoolSystem/BPC_PoolableComponent.BPC_PoolableComponent_C|SetbInPool (Actor|GetComponentbyClass InActor "/Game/RuntimeSurvival/Blueprints/PoolSystem/BPC_PoolableComponent.BPC_PoolableComponent_C") true)
              (return))))))
    (else
      (Development|PrintString "Poolable 아니면서...왜 풀링 요청을 하셨을까.."))))

(fn GetActorinPoolInterface
  (params (InActorClassType :type Actor%20Class%20Reference) (InActorLocation :type Vector :default "0, 0, 0"))
  (bind _outactor (CallFunction|GetActorinPool InActorClassType InActorLocation))
  (return _outactor))