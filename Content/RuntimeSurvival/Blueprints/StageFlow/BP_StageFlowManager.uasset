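; Stage flow manager that runs the survival countdown, boss encounter, portal and game-clear sequence.
; A looping one-second timer set on BeginPlay drives the stage clock, with remaining time pushed to the HUD through interface messages.
; When time runs out, it spawns the boss once at a placed marker and updates the goal text.
; Boss-death and portal dispatchers are bound to chain portal spawning and the player controller's clear message.
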(event EventBeginPlay
  (Utilities|Time|SetTimerbyEvent (EventDispatchers|CreateEvent :!event AccumulateStageTime) 1.0 true))

(event Collision|EventActorBeginOverlap
  (params (OtherActor :type Actor%20Object%20Reference)))

(event EventTick
  (params (DeltaSeconds :type Float%20%28single-precision%29)))

(fn ConstructionScript)

(fn AccumulateStageTime
  (Variables|Default|SetStageAccTime (+ (Variables|Default|GetStageAccTime) 1.0))
  (bind _output_get (LocalVariables|SetRemainTime (Math|Float|Max(Float) (- (Variables|Default|GetStageDuration) (Variables|Default|GetStageAccTime)) 0.0)))
  (Class|BPIPlayerHUD|UpdateRemainTimeInterface(Message) (HUD|GetHUD (Game|GetPlayerController 0)) (Math|Float|Truncate _output_get))
  (if (>= (Variables|Default|GetStageAccTime) (Variables|Default|GetStageDuration))
    (if (not (Variables|Default|GetbBossSpawned))
      (CallFunction|SpawnBoss)
      (Variables|Default|SetbBossSpawned true))))

(fn SpawnBoss
  (bind _returnvalue (Game|GetPlayerController 0))
  (bind _returnvalue_2 (HUD|GetHUD _returnvalue))
  (bind _returnvalue_3 (Game|SpawnActorfromClass "/Game/RuntimeSurvival/Blueprints/Boss/BP_Enemy_Boss.BP_Enemy_Boss_C" (Transformation|GetActorTransform (Variables|Default|GetBossSpawnLocation)) "AlwaysSpawn" "MultiplyWithRoot" 0 0))
  (EventDispatchers|BindEventtoOnBossDead _returnvalue_3 (EventDispatchers|CreateEvent :!event SpawnPortal))
  (Class|BPIPlayerHUD|UpdateRemainTimeInterface(Message) _returnvalue_2)
  (Class|BPIPlayerHUD|UpdateGoalTextInterface(Message) _returnvalue_2 (Utilities|Text|FormatText "광기의 런타임 보스가 나타났다 !  
보스를 물리치면 현실 세계로 돌아가는 포탈이 생긴다 ! 
런타임 보스를 죽이고 포탈을 찾자 !")))

(fn SpawnPortal
  (bind _bossspawnlocation (Variables|Default|GetBossSpawnLocation))
  (bind _returnvalue (Transformation|GetActorTransform _bossspawnlocation))
  (bind _returnvalue_2 (Game|SpawnActorfromClass "/Game/RuntimeSurvival/Blueprints/StageFlow/BP_Portal.BP_Portal_C" (Math|Transform|MakeTransform (Math|Vector|MakeVector (.x (.location _returnvalue)) (.y (.location _returnvalue)) 1.6e+02) (.rotation _returnvalue) (.scale _returnvalue)) "Undefined" "MultiplyWithRoot" 0 0))
  (EventDispatchers|BindEventtoOnStageClear _returnvalue_2 (EventDispatchers|CreateEvent :!event StageClear)))

(fn StageClear
  (Variables|Default|SetbStageClear true)
  (Class|BPICanHandlePlayerControlFlow|HandleGameClear(Message) (Game|GetPlayerController 0)))